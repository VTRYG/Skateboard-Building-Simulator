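; Camera Blueprint that glides between five preset viewpoints: selling, storage, assembly, store and ad.
; The MoveCamera event saves the current transform, then restarts the Movement timeline, whose alpha blends the actor toward the transform of the camera reference selected by Position.
; The actor itself moves without sweep, and no Tick or BeginPlay logic is used.
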(event Custom|MoveCamera
  (params (Position :type Integer))
  (bind _output_get (Variables|Default|SetCurrentPosition (Transformation|GetActorTransform self)))
  (bind _movement (Timeline|Movement PlayFromStart)
    (:Update
      (Transformation|SetActorTransform self (Math|Transform|Lerp(Transform) _output_get (Transformation|GetActorTransform (Utilities|Select :Index Position :Option%200 (Variables|Default|GetSellingCamera) :Option%201 (Variables|Default|GetStorageCamera) :Option%202 (Variables|Default|GetAssemblyCamera) :Option%203 (Variables|Default|GetStoreCamera) :Option%204 (Variables|Default|GetAdCamera))) _movement)))))

(event EventBeginPlay)

(event Collision|EventActorBeginOverlap
  (params (OtherActor :type Actor%20Object%20Reference)))

(event EventTick
  (params (DeltaSeconds :type Float%20%28single-precision%29)))

(fn ConstructionScript)