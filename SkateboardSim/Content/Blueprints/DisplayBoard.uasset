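; Display actor that previews an assembled skateboard, hidden until DisplayBoard receives a board to show.
; DisplayBoard applies the board's meshes and skins, seating trucks on the deck's front and back sockets and wheels on each truck's wheel socket.
; HideBoard hides the deck hierarchy and resets its three material slots to the default parts material.
; While Visible is true, touch drags rotate the actor in roll and yaw, scaled by frame time and RotationSpeed.
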(event Custom|Display%20Board
  (params (Board :type Storage%20Structure))
  (bind (_deck _deckrarity _trucks _truckrarity _wheelsmodel _wheelmodelrarity _wheelskin _wheelskinrarity _griptapeskin _griptaperarity _undersideskin) (Utilities|Struct|BreakStoredBoards (.boardinfo Board)))
  (bind _backwheels (Variables|Default|GetBackWheels))
  (bind _frontwheels (Variables|Default|GetFrontWheels))
  (bind _deck_2 (Variables|Default|GetDeck))
  (bind _fronttrucks (Variables|Default|GetFrontTrucks))
  (bind _backtrucks (Variables|Default|GetBackTrucks))
  (Rendering|SetVisibility (Variables|Default|GetDeck) true true)
  ;[0.04076 1 0.1108] Deck
  (Components|StaticMesh|SetStaticMesh _deck_2 _deck)
  (Rendering|Material|SetMaterialbyName _deck_2 "Griptape" _griptapeskin)
  (Rendering|Material|SetMaterialbyName _deck_2 "Underside" _undersideskin)
  (Rendering|Material|SetMaterialbyName _deck_2 "Board" "/Game/Materials/Decks/Parts_Inst.Parts_Inst")
  (Utilities|FlowControl|Sequence
    (:then_0
      ;[0.04076 1 0.1108] FrontTruck
      (Components|StaticMesh|SetStaticMesh _fronttrucks _trucks)
      (Transformation|SetWorldLocation _fronttrucks (Transformation|GetSocketLocation _deck_2 "front") false false)
      ;[0.04076 1 0.1108] FrontWheels
      (Components|StaticMesh|SetStaticMesh _frontwheels _wheelsmodel)
      (Rendering|Material|SetMaterial _backwheels 0 _wheelskin)
      (Transformation|SetWorldLocation _frontwheels (Transformation|GetSocketLocation _fronttrucks "wheels") false false))
    (:then_1
      ;[0.04076 1 0.1108] BackTruck
      (Components|StaticMesh|SetStaticMesh _backtrucks _trucks)
      (Transformation|SetWorldLocation _backtrucks (Transformation|GetSocketLocation _deck_2 "back") false false)
      ;[0.04076 1 0.1108] BackWheels
      (Components|StaticMesh|SetStaticMesh _backwheels _wheelsmodel)
      (Rendering|Material|SetMaterial _backwheels 0 _wheelskin)
      (Transformation|SetWorldLocation _backwheels (Transformation|GetSocketLocation _backtrucks "wheels") false false))))

(event Custom|HideBoard
  (bind _deck (Variables|Default|GetDeck))
  (Rendering|SetVisibility _deck false true)
  (Rendering|Material|SetMaterial _deck 0 "/Game/Materials/Decks/Parts_Inst.Parts_Inst")
  (Rendering|Material|SetMaterial _deck 1 "/Game/Materials/Decks/Parts_Inst.Parts_Inst")
  (Rendering|Material|SetMaterial _deck 2 "/Game/Materials/Decks/Parts_Inst.Parts_Inst"))

(event EventBeginPlay
  (Rendering|SetVisibility (Variables|Default|GetDeck) false true))

(event Input|TouchEvents|InputTouch
  (params (Location :type Vector) (FingerIndex :type ETouchIndex%20Enum))
  (bind _visible (Variables|Default|GetVisible))
  (:Pressed
    (if _visible
      (Variables|Default|SetStartLocation (CallFunction|GetTouchScreenLocation))))
  (:Moved
    (if _visible
      (Variables|Default|SetEndLocation (CallFunction|GetTouchScreenLocation))
      (Class|Actor|AddActorWorldRotation self (Math|Rotator|MakeRotator (* (.y (- (Variables|Default|GetEndLocation) (Variables|Default|GetStartLocation))) (Utilities|Time|GetWorldDeltaSeconds) (Variables|Default|GetRotationSpeed)) 0.0 (* (.x (- (Variables|Default|GetEndLocation) (Variables|Default|GetStartLocation))) (Utilities|Time|GetWorldDeltaSeconds) (Variables|Default|GetRotationSpeed) -1.0)))
      (Variables|Default|SetStartLocation (CallFunction|GetTouchScreenLocation)))))

(fn ConstructionScript)

(fn GetTouchScreenLocation
  (bind _returnvalue (Game|GetPlayerController 0))
  (bind (_locationx _locationy) (Class|PlayerController|GetInputTouchState _returnvalue "Touch1"))
  (return (Math|Vector2D|MakeVector2D _locationx _locationy)))