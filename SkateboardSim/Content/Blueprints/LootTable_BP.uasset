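; Loot box Blueprint meant to pick a part from RarityTable by weighted random and print it when OpenBox fires.
; CalculateSum accumulates the weights but returns 0.0, which becomes ValueSum, the upper limit of ChoosePart's random roll.
; The subtract-and-compare loop that would select a key is disconnected, so ChoosePart returns no chosen part as written.
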(event Custom|OpenBox
  (bind _sum (CallFunction|CalculateSum))
  (Variables|Default|SetValueSum _sum)
  (bind _part (CallFunction|ChoosePart))
  (Development|PrintString _part true true "(R=0.000000,G=0.660000,B=1.000000,A=1.000000)" 1e+01))

(fn CalculateSum
  (bind _values (Utilities|Map|Values (Variables|Default|GetRarityTable)))
  (for _array_element _values
    (LocalVariables|SetRunningTotal (+ (LocalVariables|GetRunningTotal) _array_element)))
  (return 0.0))

(fn ChoosePart
  (LocalVariables|SetRandomValue (Math|Random|RandomFloatinRange 0.0 (Variables|Default|GetValueSum)))
  (bind _keys (Utilities|Map|Keys (Variables|Default|GetRarityTable))))