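; PartsStorage is an actor that holds an item ID storage for parts and keeps it persistent through the game's save data.
; On BeginPlay it reaches the save game through BP_GI, then seeds a new save with its default storage or loads the saved PartsStorage otherwise.
; UpdateItemSavedata passes the current storage back to the game instance's SaveItemStorage to update the save.
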(event Custom|Update%20Item%20Savedata
  (Default|SaveItemStorage (Variables|Default|GetSaveBP) (Variables|Default|GetItemIDStorage)))

(event EventBeginPlay
  (bind _asbp_gi (Utilities|Casting|CastToBP_GI (Game|GetGameInstance)))
  (bind _output_get (Variables|Default|SetSaveBP _asbp_gi))
  (bind _asbp_sg (Utilities|Casting|CastToBP_SG (Variables|/Game/SaveSystem/BP_GI.BP_GI_C|GetSaveData _output_get)))
  (if (Variables|/Game/SaveSystem/BP_SG.BP_SG_C|GetNewSave _asbp_sg)
    (Default|SaveItemStorage (Variables|Default|GetSaveBP) (Variables|Default|GetItemIDStorage))
    (else
      (Variables|Default|SetItemIDStorage (Variables|/Game/SaveSystem/BP_SG.BP_SG_C|GetPartsStorage _asbp_sg)))))

(fn ConstructionScript)