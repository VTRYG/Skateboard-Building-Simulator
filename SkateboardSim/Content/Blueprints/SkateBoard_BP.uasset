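; Skateboard actor assembled from swappable deck, truck and wheel meshes, with changeable griptape, underside and wheel materials.
; Change events set meshes and materials, gating trucks on a deck and wheels on trucks.
; Changing a part re-snaps dependent parts through mesh sockets; deck swaps reapply named-slot materials only when trucks are valid.
; RotateX and RotateZ share one call setting actor roll and yaw.
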(event Custom|Change%20Deck
  (params (Deck%20Mesh :type Static%20Mesh%20Object%20Reference))
  (bind _griptape_material (Variables|Selected|GetGriptape%20Material))
  (bind _underside_material (Variables|Selected|GetUnderside%20Material))
  ;[1 1 1] Deck Mesh Generation
  (bind _output_get (Variables|Selected|SetDeck Deck%20Mesh))
  (Components|StaticMesh|SetStaticMesh (Variables|Default|GetDeck%20Mesh) _output_get)
  (Variables|Default|SetDeckOn true)
  (if (Utilities|IsValid (Variables|Selected|GetTrucks))
    (Utilities|FlowControl|Sequence
      (:then_0
        (Utilities|FlowControl|Sequence
          (:then_0
            (if (Utilities|IsValid _griptape_material)
              (Rendering|Material|SetMaterial (Variables|Default|GetDeck%20Mesh) (Rendering|Material|GetMaterialIndex (Variables|Default|GetDeck%20Mesh) "Griptape") _griptape_material)))
          (:then_1
            (if (Utilities|IsValid _underside_material)
              (Rendering|Material|SetMaterial (Variables|Default|GetDeck%20Mesh) (Rendering|Material|GetMaterialIndex (Variables|Default|GetDeck%20Mesh) "UnderSide") _underside_material)))
          (:then_2
            (Rendering|Material|SetMaterial (Variables|Default|GetDeck%20Mesh) (Rendering|Material|GetMaterialIndex (Variables|Default|GetDeck%20Mesh) "Board") "/Game/Puzzle/Meshes/BaseMaterial.BaseMaterial"))))
      (:then_1
        ;[1 1 1] Truck Mesh Generation
        (Utilities|FlowControl|Sequence
          (:then_0
            (Transformation|SetWorldLocation (Variables|Default|GetFront%20Trucks%20Mesh) (Transformation|GetSocketLocation (Variables|Default|GetDeck%20Mesh) "front") false false))
          (:then_1
            (Transformation|SetWorldLocation (Variables|Default|GetBack%20Trucks%20Mesh) (Transformation|GetSocketLocation (Variables|Default|GetDeck%20Mesh) "back") false false)
            (if (Utilities|IsValid (Variables|Selected|GetWheels))
              ;[1 1 1] Wheel Mesh Generation and texture
              (Utilities|FlowControl|Sequence
                (:then_0
                  (Transformation|SetWorldLocation (Variables|Default|GetFront%20Wheels%20Mesh) (Transformation|GetSocketLocation (Variables|Default|GetFront%20Trucks%20Mesh) "wheels") false false))
                (:then_1
                  (Transformation|SetWorldLocation (Variables|Default|GetBack%20Wheels%20Mesh) (Transformation|GetSocketLocation (Variables|Default|GetBack%20Trucks%20Mesh) "wheels") false false))))))))))

(event Custom|Change%20Wheels
  (params (Wheels%20Mesh :type Static%20Mesh%20Object%20Reference) (Wheels%20Texture :type Material%20Interface%20Object%20Reference))
  (bind _front_wheels_mesh (Variables|Default|GetFront%20Wheels%20Mesh))
  (bind _back_wheels_mesh (Variables|Default|GetBack%20Wheels%20Mesh))
  ;[1 1 1] Wheel Mesh Generation and texture
  (if (Variables|Default|GetTrucksOn)
    (bind _output_get (Variables|Selected|SetWheels Wheels%20Mesh))
    (bind _output_get_2 (Variables|Selected|SetWheels%20Material Wheels%20Texture))
    (Components|StaticMesh|SetStaticMesh _front_wheels_mesh _output_get)
    (Rendering|Material|SetMaterial _front_wheels_mesh 0 _output_get_2)
    (Components|StaticMesh|SetStaticMesh _back_wheels_mesh _output_get)
    (Rendering|Material|SetMaterial _back_wheels_mesh 0 _output_get_2)
    (Utilities|FlowControl|Sequence
      (:then_0
        (Transformation|SetWorldLocation (Variables|Default|GetFront%20Wheels%20Mesh) (Transformation|GetSocketLocation (Variables|Default|GetFront%20Trucks%20Mesh) "wheels") false false))
      (:then_1
        (Transformation|SetWorldLocation (Variables|Default|GetBack%20Wheels%20Mesh) (Transformation|GetSocketLocation (Variables|Default|GetBack%20Trucks%20Mesh) "wheels") false false)))))

(event Custom|Change%20Trucks
  (params (Truck%20Mesh :type Static%20Mesh%20Object%20Reference))
  (bind _deck_mesh (Variables|Default|GetDeck%20Mesh))
  ;[1 1 1] Truck Mesh Generation
  (if (Variables|Default|GetDeckOn)
    (Variables|Default|SetTrucksOn true)
    (bind _output_get (Variables|Selected|SetTrucks Truck%20Mesh))
    (Components|StaticMesh|SetStaticMesh (Variables|Default|GetFront%20Trucks%20Mesh) _output_get)
    (Components|StaticMesh|SetStaticMesh (Variables|Default|GetBack%20Trucks%20Mesh) _output_get)
    (Utilities|FlowControl|Sequence
      (:then_0
        (Transformation|SetWorldLocation (Variables|Default|GetFront%20Trucks%20Mesh) (Transformation|GetSocketLocation _deck_mesh "front") false false))
      (:then_1
        (Transformation|SetWorldLocation (Variables|Default|GetBack%20Trucks%20Mesh) (Transformation|GetSocketLocation _deck_mesh "back") false false)
        (if (Utilities|IsValid (Variables|Selected|GetWheels))
          ;[1 1 1] Wheel Mesh Generation and texture
          (Utilities|FlowControl|Sequence
            (:then_0
              (Transformation|SetWorldLocation (Variables|Default|GetFront%20Wheels%20Mesh) (Transformation|GetSocketLocation (Variables|Default|GetFront%20Trucks%20Mesh) "wheels") false false))
            (:then_1
              (Transformation|SetWorldLocation (Variables|Default|GetBack%20Wheels%20Mesh) (Transformation|GetSocketLocation (Variables|Default|GetBack%20Trucks%20Mesh) "wheels") false false))))))))

(event Custom|Rotate%20X
  (params (X :type Float%20%28single-precision%29))
  (Transformation|SetActorRotation self (Math|Rotator|MakeRotator X 0.0 (stale Custom|Rotate%20Z Z))))

(event Custom|Change%20GripTape
  (params (Griptape%20Texture :type Material%20Interface%20Object%20Reference))
  (bind _deck_mesh (Variables|Default|GetDeck%20Mesh))
  ;[1 1 1] Deck Griptape Material Generation
  (if (Utilities|IsValid (Variables|Selected|GetDeck))
    (bind _output_get (Variables|Selected|SetGriptape%20Material Griptape%20Texture))
    (Rendering|Material|SetMaterial _deck_mesh (Rendering|Material|GetMaterialIndex _deck_mesh "Griptape") _output_get)))

(event Custom|Rotate%20Z
  (params (Z :type Float%20%28single-precision%29))
  (Transformation|SetActorRotation self (Math|Rotator|MakeRotator (stale Custom|Rotate%20X X) 0.0 Z)))

(event Custom|Change%20Underside
  (params (Underside%20Texture :type Material%20Interface%20Object%20Reference))
  (bind _deck_mesh (Variables|Default|GetDeck%20Mesh))
  ;[1 1 1] Deck Underside Material Generation
  (if (Utilities|IsValid (Variables|Selected|GetDeck))
    (bind _output_get (Variables|Selected|SetUnderside%20Material Underside%20Texture))
    (Rendering|Material|SetMaterial _deck_mesh (Rendering|Material|GetMaterialIndex _deck_mesh "UnderSide") _output_get)))

(fn ConstructionScript)