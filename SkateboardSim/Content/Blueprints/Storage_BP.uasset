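; Skateboard storage actor that displays saved boards across ten slots and persists changes through the game instance.
; BeginPlay loads the Storage array from the save game into Used and SlotInfo and spawns meshes for occupied slots.
; StoreBoard saves a board and builds its deck, trucks and wheels at runtime as socket-attached static mesh components with per-board materials.
; RemoveBoard clears the slot, saves, and destroys that component hierarchy by child index.
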(event Custom|Store%20Board
  (params (Board :type Stored%20Boards%20Structure) (Slot%20Number :type Integer))
  (bind _used (Variables|Default|GetUsed))
  (bind _slot_info (Variables|Default|GetSlot%20Info))
  (bind _output (Utilities|Array|Get(acopy) _slot_info Slot%20Number))
  (bind (_deck _deckrarity _trucks _truckrarity _wheelsmodel _wheelmodelrarity _wheelskin _wheelskinrarity _griptapeskin _griptaperarity _undersideskin) (Utilities|Struct|BreakStoredBoards _output))
  (if (not (Utilities|Array|Get(acopy) _used Slot%20Number))
    (Utilities|Array|SetArrayElem _slot_info Slot%20Number Board)
    (Utilities|Array|SetArrayElem (Variables|Default|GetStorage) Slot%20Number (Utilities|Struct|MakeStorage true _output))
    (Utilities|Array|SetArrayElem _used Slot%20Number true)
    (Default|SaveStorage (Variables|Default|GetSaveBP) (Variables|Default|GetStorage))
    ;[0.04076 1 0.1108] Deck
    (bind _returnvalue (AddComponent|AddStaticMeshComponent false))
    (Components|StaticMesh|SetStaticMesh _returnvalue _deck)
    (Rendering|Material|SetMaterialbyName _returnvalue "Griptape" _griptapeskin)
    (Rendering|Material|SetMaterialbyName _returnvalue "Underside" _undersideskin)
    (Transformation|AttachComponentToComponent _returnvalue (Utilities|Array|Get(acopy) (Variables|Default|GetSlot) Slot%20Number) "" "KeepRelative" "KeepRelative" "KeepRelative" false)
    (Utilities|FlowControl|Sequence
      (:then_0
        ;[0.04076 1 0.1108] FrontTruck
        (bind _returnvalue_2 (AddComponent|AddStaticMeshComponent false))
        (Components|StaticMesh|SetStaticMesh _returnvalue_2 _trucks)
        (Transformation|AttachComponentToComponent _returnvalue_2 _returnvalue "Front" "KeepRelative" "KeepRelative" "KeepRelative" false)
        ;[0.04076 1 0.1108] FrontWheels
        (bind _returnvalue_3 (AddComponent|AddStaticMeshComponent false))
        (Components|StaticMesh|SetStaticMesh _returnvalue_3 _wheelsmodel)
        (Rendering|Material|SetMaterial _returnvalue_3 0 _wheelskin)
        (Transformation|AttachComponentToComponent _returnvalue_3 _returnvalue_2 "Wheels" "KeepRelative" "KeepRelative" "KeepRelative" false))
      (:then_1
        ;[0.04076 1 0.1108] BackTruck
        (bind _returnvalue_4 (AddComponent|AddStaticMeshComponent false))
        (Components|StaticMesh|SetStaticMesh _returnvalue_4 _trucks)
        (Transformation|AttachComponentToComponent _returnvalue_4 _returnvalue "Back" "KeepRelative" "KeepRelative" "KeepRelative" false)
        ;[0.04076 1 0.1108] BackWheels
        (bind _returnvalue_5 (AddComponent|AddStaticMeshComponent false))
        (Components|StaticMesh|SetStaticMesh _returnvalue_5 _wheelsmodel)
        (Rendering|Material|SetMaterial _returnvalue_5 0 _wheelskin)
        (Transformation|AttachComponentToComponent _returnvalue_5 _returnvalue_4 "Wheels" "KeepRelative" "KeepRelative" "KeepRelative" false)))))

(event Custom|RemoveBoard
  (params (Slot%20Number :type Integer))
  (bind _slot (Variables|Default|GetSlot))
  (bind _used (Variables|Default|GetUsed))
  (bind _output (Utilities|Array|Get(acopy) _slot Slot%20Number))
  (bind _returnvalue (Components|GetChildComponent _output 0))
  (bind _returnvalue_2 (Components|GetChildComponent _returnvalue 1))
  (bind _returnvalue_3 (Components|GetChildComponent _returnvalue 0))
  (if (Utilities|Array|Get(acopy) _used Slot%20Number)
    (Utilities|Array|SetArrayElem _used Slot%20Number false)
    (Utilities|Array|SetArrayElem :TargetArray (Variables|Default|GetSlot%20Info) :Index Slot%20Number)
    (Utilities|Array|SetArrayElem (Variables|Default|GetStorage) Slot%20Number (Utilities|Struct|MakeStorage false "(Deck_3_07921BFE425CC83915399B9E7DBF1AC8=None,DeckRarity_17_B68A13CB4E463CCDED1CD4A4B5BC4CBD=NewEnumerator0,Trucks_5_323A3C4E4A3469B5C25470AEF30F7864=None,TruckRarity_19_0206BE8B4BD82F51666CA8BDC670A73D=NewEnumerator0,WheelsModel_7_B2FDD1284A09C064DE9CE19C449164E6=None,WheelModelRarity_24_1E934EA0412F6AA7DABE7F971144EA39=NewEnumerator0,WheelSkin_10_83AEC3744776C1005D397AA6F776EFBF=None,WheelSkinRarity_25_2F7CD5F246E235B21BBF419BC34F8FE4=NewEnumerator0,GriptapeSkin_12_A482E79245CA37F717D17EA678216B05=None,GriptapeRarity_27_4C54D3454974A62B83B49FB34F6C8860=NewEnumerator0,UndersideSkin_14_0D74F6634DAF9974C243898FF3D40A4A=None,UndersideRarity_29_FA8666A14254CE3F92B023A78B5ECF39=NewEnumerator0)"))
    (Default|SaveStorage (Variables|Default|GetSaveBP) (Variables|Default|GetStorage))
    (Components|DestroyComponent (Components|GetChildComponent _returnvalue_2 0))
    (Components|DestroyComponent (Components|GetChildComponent _returnvalue_3 0))
    (Components|DestroyComponent _returnvalue_2)
    (Components|DestroyComponent _returnvalue_3)
    (Components|DestroyComponent _returnvalue)))

(event EventBeginPlay
  (bind _asbp_gi (Utilities|Casting|CastToBP_GI (Game|GetGameInstance)))
  (bind _output_get (Variables|Default|SetSaveBP _asbp_gi))
  (bind _asbp_sg (Utilities|Casting|CastToBP_SG (Variables|/Game/SaveSystem/BP_GI.BP_GI_C|GetSaveData _output_get)))
  (bind _output_get_2 (Variables|Default|SetStorage (Variables|/Game/SaveSystem/BP_SG.BP_SG_C|GetStorage _asbp_sg)))
  (for (_array_element _array_index) _output_get_2
    (Utilities|Array|SetArrayElem (Variables|Default|GetUsed) _array_index (.slotused _array_element))
    (Utilities|Array|SetArrayElem (Variables|Default|GetSlot%20Info) _array_index (.boardinfo _array_element))
    (for (_array_element_2 _array_index_2) (Variables|Default|GetStorage)
      (if (.slotused _array_element_2)
        ;[0.04076 1 0.1108] Deck
        (bind _returnvalue (AddComponent|AddStaticMeshComponent false))
        (Components|StaticMesh|SetStaticMesh _returnvalue (.Deck (Utilities|Struct|BreakStoredBoards (.boardinfo _array_element_2))))
        (Rendering|Material|SetMaterialbyName _returnvalue "Griptape" (.GriptapeSkin (Utilities|Struct|BreakStoredBoards (.boardinfo _array_element_2))))
        (Rendering|Material|SetMaterialbyName _returnvalue "Underside" (.UndersideSkin (Utilities|Struct|BreakStoredBoards (.boardinfo _array_element_2))))
        (Transformation|AttachComponentToComponent _returnvalue (Utilities|Array|Get(acopy) (Variables|Default|GetSlot) _array_index_2) "" "KeepRelative" "KeepRelative" "KeepRelative" false)
        (Utilities|FlowControl|Sequence
          (:then_0
            ;[0.04076 1 0.1108] FrontTruck
            (bind _returnvalue_2 (AddComponent|AddStaticMeshComponent false))
            (Components|StaticMesh|SetStaticMesh _returnvalue_2 (.Trucks (Utilities|Struct|BreakStoredBoards (.boardinfo _array_element_2))))
            (Transformation|AttachComponentToComponent _returnvalue_2 _returnvalue "Front" "KeepRelative" "KeepRelative" "KeepRelative" false)
            ;[0.04076 1 0.1108] FrontWheels
            (bind _returnvalue_3 (AddComponent|AddStaticMeshComponent false))
            (Components|StaticMesh|SetStaticMesh _returnvalue_3 (.WheelsModel (Utilities|Struct|BreakStoredBoards (.boardinfo _array_element_2))))
            (Rendering|Material|SetMaterial _returnvalue_3 0 (.WheelSkin (Utilities|Struct|BreakStoredBoards (.boardinfo _array_element_2))))
            (Transformation|AttachComponentToComponent _returnvalue_3 _returnvalue_2 "Wheels" "KeepRelative" "KeepRelative" "KeepRelative" false))
          (:then_1
            ;[0.04076 1 0.1108] BackTruck
            (bind _returnvalue_4 (AddComponent|AddStaticMeshComponent false))
            (Components|StaticMesh|SetStaticMesh _returnvalue_4 (.Trucks (Utilities|Struct|BreakStoredBoards (.boardinfo _array_element_2))))
            (Transformation|AttachComponentToComponent _returnvalue_4 _returnvalue "Back" "KeepRelative" "KeepRelative" "KeepRelative" false)
            ;[0.04076 1 0.1108] BackWheels
            (bind _returnvalue_5 (AddComponent|AddStaticMeshComponent false))
            (Components|StaticMesh|SetStaticMesh _returnvalue_5 (.WheelsModel (Utilities|Struct|BreakStoredBoards (.boardinfo _array_element_2))))
            (Rendering|Material|SetMaterial _returnvalue_5 0 (.WheelSkin (Utilities|Struct|BreakStoredBoards (.boardinfo _array_element_2))))
            (Transformation|AttachComponentToComponent _returnvalue_5 _returnvalue_4 "Wheels" "KeepRelative" "KeepRelative" "KeepRelative" false)))))))

(fn ConstructionScript
  (Variables|Default|SetSlot (Utilities|Array|MakeArray (Variables|Default|GetSlot1) (Variables|Default|GetSlot2) (Variables|Default|GetSlot3) (Variables|Default|GetSlot4) (Variables|Default|GetSlot5) (Variables|Default|GetSlot6) (Variables|Default|GetSlot7) (Variables|Default|GetSlot8) (Variables|Default|GetSlot9) (Variables|Default|GetSlot10))))