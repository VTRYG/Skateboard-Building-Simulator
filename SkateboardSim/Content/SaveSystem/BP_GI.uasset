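; BP_GI is a game instance that manages the game's save data through a BP_SG save object in a single default slot.
; On Init it loads the existing save, or creates and writes a new one.
; Events save or reload the whole object, and SaveStorage copies storage data into it before writing.
; LoadStorage only reloads the save object, the same as LoadGame.
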(event Custom|SaveGame
  (params (NewParam :type Struct%20Board%20Types%20Structure))
  (Utilities|Casting|CastToBP_SG (Variables|Default|GetSaveData))
  (bind _returnvalue (SaveGame|SaveGametoSlot (Variables|Default|GetSaveData) (Variables|Default|GetDefaultSlot)))
  (if _returnvalue
    _))

(event Custom|LoadGame
  (bind _returnvalue (SaveGame|LoadGamefromSlot (Variables|Default|GetDefaultSlot)))
  (Variables|Default|SetSaveData _returnvalue))

(event Custom|LoadStorage
  (bind _returnvalue (SaveGame|LoadGamefromSlot (Variables|Default|GetDefaultSlot)))
  (Variables|Default|SetSaveData _returnvalue))

(event Custom|SaveStorage
  (params (Storage :type Array%20of%20Storage%20Structures))
  (bind _asbp_sg (Utilities|Casting|CastToBP_SG (Variables|Default|GetSaveData)))
  (Variables|/Game/SaveSystem/BP_SG.BP_SG_C|SetStorage _asbp_sg Storage)
  (bind _returnvalue (SaveGame|SaveGametoSlot (Variables|Default|GetSaveData) (Variables|Default|GetDefaultSlot)))
  (if _returnvalue
    _))

(event EventInit
  (bind _returnvalue (SaveGame|DoesSaveGameExist (Variables|Default|GetDefaultSlot)))
  (if _returnvalue
    (bind _returnvalue_2 (SaveGame|LoadGamefromSlot (Variables|Default|GetDefaultSlot)))
    (Variables|Default|SetSaveData _returnvalue_2)
    (else
      (bind _returnvalue_3 (SaveGame|CreateSaveGameObject "/Game/SaveSystem/BP_SG.BP_SG_C"))
      (Variables|Default|SetSaveData _returnvalue_3)
      (bind _returnvalue_4 (SaveGame|SaveGametoSlot (Variables|Default|GetSaveData) (Variables|Default|GetDefaultSlot)))
      (if _returnvalue_4
        _))))