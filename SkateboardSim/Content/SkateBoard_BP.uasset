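; Customisable skateboard actor that swaps deck, truck and wheel meshes and rotates on roll and yaw through events.
; Part changes cascade through sockets: trucks snap to the deck's "front" and "back", wheels to each truck's "wheels".
; Wheel, grip tape and underside events step through material lists by index, ignoring their texture inputs.
; Grip tape and underside materials occupy separate slots on the deck mesh.
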(event Custom|Change%20Deck
  (params (Deck%20Mesh :type Static%20Mesh%20Object%20Reference))
  ;[1 1 1] Deck Mesh Generation
  (bind _output_get (Variables|Default|SetDeck Deck%20Mesh))
  (Components|StaticMesh|SetStaticMesh (Variables|Default|GetDeck%20Mesh) _output_get)
  (if (Utilities|IsValid (Variables|Default|GetTrucks))
    ;[1 1 1] Truck Mesh Generation
    (Utilities|FlowControl|Sequence
      (:then_0
        (Transformation|SetWorldLocation (Variables|Default|GetFront%20Trucks%20Mesh) (Transformation|GetSocketLocation (Variables|Default|GetDeck%20Mesh) "front") false false))
      (:then_1
        (Transformation|SetWorldLocation (Variables|Default|GetBack%20Trucks%20Mesh) (Transformation|GetSocketLocation (Variables|Default|GetDeck%20Mesh) "back") false false)
        (if (Utilities|IsValid (Variables|Default|GetWheels))
          ;[1 1 1] Wheel Mesh Generation and texture
          (Utilities|FlowControl|Sequence
            (:then_0
              (Transformation|SetWorldLocation (Variables|Default|GetFront%20Wheels%20Mesh) (Transformation|GetSocketLocation (Variables|Default|GetFront%20Trucks%20Mesh) "wheels") false false))
            (:then_1
              (Transformation|SetWorldLocation (Variables|Default|GetBack%20Wheels%20Mesh) (Transformation|GetSocketLocation (Variables|Default|GetBack%20Trucks%20Mesh) "wheels") false false))))))))

(event Custom|Change%20Wheels
  (params (Wheels%20Mesh :type Static%20Mesh%20Object%20Reference) (Wheels%20Texture :type Material%20Interface%20Object%20Reference))
  (bind _front_wheels_mesh (Variables|Default|GetFront%20Wheels%20Mesh))
  (bind _back_wheels_mesh (Variables|Default|GetBack%20Wheels%20Mesh))
  (bind _wheels_list (Variables|Default|GetWheels%20List))
  (if (>= (Variables|Default|GetCurrent%20Wheel) (Utilities|Array|Length _wheels_list))
    (Variables|Default|SetCurrent%20Wheel 0)
    (else
      (Variables|Default|SetCurrent%20Wheel (+ (Variables|Default|GetCurrent%20Wheel) 1))))
  ;[1 1 1] Wheel Mesh Generation and texture
  (bind _output_get (Variables|Default|SetWheels Wheels%20Mesh))
  (bind _output_get_2 (Variables|Default|SetWheels%20Material (Utilities|Array|Get(acopy) _wheels_list (Variables|Default|GetCurrent%20Wheel))))
  (Components|StaticMesh|SetStaticMesh _front_wheels_mesh _output_get)
  (Rendering|Material|SetMaterial _front_wheels_mesh 0 _output_get_2)
  (Components|StaticMesh|SetStaticMesh _back_wheels_mesh _output_get)
  (Rendering|Material|SetMaterial _back_wheels_mesh 0 _output_get_2)
  (Utilities|FlowControl|Sequence
    (:then_0
      (Transformation|SetWorldLocation (Variables|Default|GetFront%20Wheels%20Mesh) (Transformation|GetSocketLocation (Variables|Default|GetFront%20Trucks%20Mesh) "wheels") false false))
    (:then_1
      (Transformation|SetWorldLocation (Variables|Default|GetBack%20Wheels%20Mesh) (Transformation|GetSocketLocation (Variables|Default|GetBack%20Trucks%20Mesh) "wheels") false false))))

(event Custom|Change%20Trucks
  (params (Truck%20Mesh :type Static%20Mesh%20Object%20Reference))
  (bind _deck_mesh (Variables|Default|GetDeck%20Mesh))
  ;[1 1 1] Truck Mesh Generation
  (bind _output_get (Variables|Default|SetTrucks Truck%20Mesh))
  (Components|StaticMesh|SetStaticMesh (Variables|Default|GetFront%20Trucks%20Mesh) _output_get)
  (Components|StaticMesh|SetStaticMesh (Variables|Default|GetBack%20Trucks%20Mesh) _output_get)
  (Utilities|FlowControl|Sequence
    (:then_0
      (Transformation|SetWorldLocation (Variables|Default|GetFront%20Trucks%20Mesh) (Transformation|GetSocketLocation _deck_mesh "front") false false))
    (:then_1
      (Transformation|SetWorldLocation (Variables|Default|GetBack%20Trucks%20Mesh) (Transformation|GetSocketLocation _deck_mesh "back") false false)
      (if (Utilities|IsValid (Variables|Default|GetWheels))
        ;[1 1 1] Wheel Mesh Generation and texture
        (Utilities|FlowControl|Sequence
          (:then_0
            (Transformation|SetWorldLocation (Variables|Default|GetFront%20Wheels%20Mesh) (Transformation|GetSocketLocation (Variables|Default|GetFront%20Trucks%20Mesh) "wheels") false false))
          (:then_1
            (Transformation|SetWorldLocation (Variables|Default|GetBack%20Wheels%20Mesh) (Transformation|GetSocketLocation (Variables|Default|GetBack%20Trucks%20Mesh) "wheels") false false)))))))

(event Custom|Rotate%20X
  (params (X :type Float%20%28single-precision%29))
  (Transformation|SetActorRotation self (Math|Rotator|MakeRotator X 0.0 (stale Custom|Rotate%20Z Z))))

(event Custom|Change%20GripTape
  (params (Griptape%20Texture :type Material%20Interface%20Object%20Reference))
  (bind _griptape_list (Variables|Default|GetGriptape%20List))
  (if (>= (Variables|Default|GetCurrent%20Griptape) (Utilities|Array|Length _griptape_list))
    (Variables|Default|SetCurrent%20Griptape 0)
    (else
      (Variables|Default|SetCurrent%20Griptape (+ (Variables|Default|GetCurrent%20Griptape) 1))))
  ;[1 1 1] Deck Griptape Material Generation
  (if (Utilities|IsValid (Variables|Default|GetDeck))
    (bind _output_get (Variables|Default|SetGriptape%20Material (Utilities|Array|Get(acopy) _griptape_list (Variables|Default|GetCurrent%20Griptape))))
    (Rendering|Material|SetMaterial (Variables|Default|GetDeck%20Mesh) 0 _output_get)))

(event Custom|Rotate%20Z
  (params (Z :type Float%20%28single-precision%29))
  (Transformation|SetActorRotation self (Math|Rotator|MakeRotator (stale Custom|Rotate%20X X) 0.0 Z)))

(event Custom|Change%20Underside
  (params (Underside%20Texture :type Material%20Interface%20Object%20Reference))
  (bind _underside_list (Variables|Default|GetUnderside%20List))
  (if (>= (Variables|Default|GetCurrent%20Underbody) (Utilities|Array|Length _underside_list))
    (Variables|Default|SetCurrent%20Underbody 0)
    (else
      (Variables|Default|SetCurrent%20Underbody (+ (Variables|Default|GetCurrent%20Underbody) 1))))
  ;[1 1 1] Deck Underside Material Generation
  (if (Utilities|IsValid (Variables|Default|GetDeck))
    (bind _output_get (Variables|Default|SetUnderside%20Material (Utilities|Array|Get(acopy) _underside_list (Variables|Default|GetCurrent%20Underbody))))
    (Rendering|Material|SetMaterial (Variables|Default|GetDeck%20Mesh) 2 _output_get)))

(fn ConstructionScript)